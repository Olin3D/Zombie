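; VR game mode that runs a wave-based zombie survival loop, starting two seconds after play begins.
; Each wave spawns twice its number in BaseZombie AI at random reachable points around the player, facing them, paced by a looping timer.
; Spawned zombies are tracked in LiveZombies, which timer-driven checks poll until all are dead.
; A cleared wave starts the next; after the last, victory repeatedly prints "Winner".
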(event Custom|SpawnZombie
  (bind _returnvalue (Game|Player|GetPlayerPawn 0))
  (bind _returnvalue_2 (Transformation|GetActorLocation _returnvalue))
  (if (> (Variables|Default|GetZombiesToSpawn) 0)
    (bind _output_get (Variables|Default|SetSpawnLocation (.RandomLocation (AI|Navigation|GetRandomReachablePointinRadius _returnvalue_2 2.5e+03))))
    (Development|PrintString "Spawn")
    (bind _returnvalue_3 (AI|SpawnAIFromClass "/Game/FirstPersonBP/Blueprints/BaseZombie.BaseZombie_C" 0 _output_get (Math|Rotator|FindLookatRotation _output_get _returnvalue_2) true))
    (Variables|Default|SetZombiesToSpawn (- (Variables|Default|GetZombiesToSpawn) 1))
    (Utilities|Array|AddUnique (Variables|Default|GetLiveZombies) _returnvalue_3)
    (Utilities|Time|SetTimerbyEvent (delegate Custom|SpawnZombie) (Variables|Default|GetTimeBetweenSpawns) true)
    (else
      (CallFunction|CheckforWave))))

(event Custom|NewWave
  (if (< (Variables|Default|GetCurrentWave) (Variables|Default|GetNumberOfWaves))
    (Variables|Default|SetCurrentWave (+ (Variables|Default|GetCurrentWave) 1))
    (Variables|Default|SetZombiesToSpawn (* (Variables|Default|GetCurrentWave) 2))
    (CallFunction|SpawnZombie)
    (Development|PrintString "Wave Started")
    (else
      (CallFunction|CheckforVictory))))

(event Custom|CheckForWave
  (Variables|Default|SetWaveComplete true)
  (for _array_element (Variables|Default|GetLiveZombies)
    (if (Variables|/Game/FirstPersonBP/Blueprints/BaseZombie.BaseZombie_C|GetIsAlive _array_element)
      (Variables|Default|SetWaveComplete false)))
  (if (Variables|Default|GetWaveComplete)
    (CallFunction|NewWave)
    (else
      (Utilities|Time|SetTimerbyEvent (delegate Custom|CheckForWave) 1.0))))

(event Custom|CheckForVictory
  (Variables|Default|SetHasWon true)
  (for _array_element (Variables|Default|GetLiveZombies)
    (if (Variables|/Game/FirstPersonBP/Blueprints/BaseZombie.BaseZombie_C|GetIsAlive _array_element)
      (Variables|Default|SetHasWon false)))
  (if (Variables|Default|GetHasWon) :!label _label
    (Development|PrintString "Winner")
    (Utilities|FlowControl|Delay 1.0)
    (goto _label)
    (else
      (Utilities|Time|SetTimerbyEvent (delegate Custom|CheckForVictory) 1.0))))

(event EventTick
  (params (DeltaSeconds :type Float%20%28single-precision%29)))

(event EventBeginPlay
  (Utilities|FlowControl|Delay 2.0)
  (CallFunction|NewWave))

(fn ConstructionScript)